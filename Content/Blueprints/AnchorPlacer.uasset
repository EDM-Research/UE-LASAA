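; Actor that places paired internal and external tracking anchors from camera poses received over OSC, then aligns them.
; An OSC server receives messages; after a place input, the next one is used if tracking state is zero and enough matches are reported.
; Its 4x4 matrix is converted from OpenCV to Unreal, spawning EXT there and INT at the player camera.
; The pair is linked and the alignment component realigns; another input resets all anchors.
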(event `EnhancedInput|/LASAA/InputActions/IA_ResetAnchors`
  (params (ActionValue :type Boolean) (ElapsedSeconds :type "Float (double-precision)") (TriggeredSeconds :type "Float (double-precision)") (InputAction :type "InputAction Object Reference" :default "/LASAA/InputActions/IA_ResetAnchors.IA_ResetAnchors"))
  ;[1 1 1] Reset all anchors
  (:`Triggered`
    (`Anchor.resetAnchors`)))

(event `EnhancedInput|/LASAA/InputActions/IA_PlaceAnchor`
  (params (ActionValue :type Boolean) (ElapsedSeconds :type "Float (double-precision)") (TriggeredSeconds :type "Float (double-precision)") (InputAction :type "InputAction Object Reference" :default "/LASAA/InputActions/IA_PlaceAnchor.IA_PlaceAnchor"))
  ;[1 1 1] Place a new anchor
  (:`Triggered`
    (set `self.PlaceAnchor` true)))

(event `self.ReceiveBeginPlay`
  ;[1 1 1] Setup
  (bind _returnvalue (`OSCManager.CreateOSCServer` "" 8001 false true "" self))
  (add `OSCServer.OnOscMessageReceived` _returnvalue (delegate `CustomEvent`))
  (bind _returnvalue_2 (`AddComponent|NODE_AddAlignmentComponent-2` :`anchorBuffer` (`self.AnchorBuffer`)))
  (`AlignmentComponent.configureAlignmentComponent` _returnvalue_2 (`self.INTAnchorClass`) (`self.EXTAnchorClass`) 1 false)
  (set `self.MinNumberMatches` (`self.MinNumberMatches`)))

(event `CustomEvent`
  (params (Message :type "OSCMessage Structure (by ref)") (IPAddress :type String) (Port :type Integer))
  ;[1 1 1] On OSC received
  ;;[1 1 1] Only continue when an anchor needs to be placed, and if tracking state is 0
  (if (`self.PlaceAnchor`)
    (set `self.PlaceAnchor` false)
    (bind _value (`OSCManager.GetInt32` Message))
    (if (== _value 0)
      (bind _transform (`self.TransformOSCPackage` Message))
      ;;[1 1 1] Make sure enough matches were found
      (`OSCManager.GetInt32` Message 17) ; KFid
      (bind _value_2 (`OSCManager.GetInt32` Message 18)) ; nrMatches
      (if (> _value_2 (`self.MinNumberMatches`))
        ;;[1 1 1] Place both INT and EXT anchors
        (bind _returnvalue (`|SpawnActorFromClass` (`self.INTAnchorClass`) (`SceneComponent.K2_GetComponentToWorld` (`self.GetComponentByClass` (`GameplayStatics.GetPlayerPawn` 0) "/Script/Engine.CameraComponent")) "AlwaysSpawn" "MultiplyWithRoot" null null))
        (`Anchor.createAnchor` _returnvalue _transform)
        (bind _returnvalue_2 (`|SpawnActorFromClass` (`self.EXTAnchorClass`) _transform "AlwaysSpawn" "MultiplyWithRoot" null null))
        (`self.K2_AttachToActor` _returnvalue_2 self "None" "KeepRelative" "KeepRelative" "KeepRelative" false)
        (`Anchor.setExtPairAndCalibrationOffset` _returnvalue _returnvalue_2)
        (`AlignmentComponent.align` (stale `self.ReceiveBeginPlay` _returnvalue_2))
        (else
          (`KismetSystemLibrary.PrintString` " \n \n \n \n \n \n                                                                                                                                                                                                                                                                                                                                                                                                                     Not enough matches found"))))))

(fn `TransformOSCPackage`
  (params (Message :type "OSCMessage Structure (by ref)"))
  (returns (Transform :type "Transform Structure"))
  (bind _value (`OSCManager.GetFloat` Message 1))
  (bind _value_2 (`OSCManager.GetFloat` Message 2))
  (bind _value_3 (`OSCManager.GetFloat` Message 3))
  (bind _value_4 (`OSCManager.GetFloat` Message 4))
  (bind _value_5 (`OSCManager.GetFloat` Message 5))
  (bind _value_6 (`OSCManager.GetFloat` Message 6))
  (bind _value_7 (`OSCManager.GetFloat` Message 7))
  (bind _value_8 (`OSCManager.GetFloat` Message 8))
  (bind _value_9 (`OSCManager.GetFloat` Message 9))
  (bind _value_10 (`OSCManager.GetFloat` Message 10))
  (bind _value_11 (`OSCManager.GetFloat` Message 11))
  (bind _value_12 (`OSCManager.GetFloat` Message 12))
  (bind _value_13 (`OSCManager.GetFloat` Message 13))
  (bind _value_14 (`OSCManager.GetFloat` Message 14))
  (bind _value_15 (`OSCManager.GetFloat` Message 15))
  (bind _value_16 (`OSCManager.GetFloat` Message 16))
  (bind _returnvalue (`Helper.ConvertOpenCVToUnreal` (`KismetMathLibrary.Conv_MatrixToTransform` (`KismetMathLibrary.Matrix_GetTransposed` (make `Matrix` (make `Plane` (* 100.0 _value_4) _value _value_2 _value_3) (make `Plane` (* 100.0 _value_8) _value_5 _value_6 _value_7) (make `Plane` (* 100.0 _value_12) _value_9 _value_10 _value_11) (make `Plane` _value_16 _value_13 _value_14 _value_15))))))
  (return _returnvalue))

(fn `UserConstructionScript`)