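; Base anchor placer that creates paired INT/EXT anchors and aligns them through an alignment component configured at BeginPlay.
; Input actions reset anchors or only raise a PlaceAnchor flag; nothing here reads that flag or calls Align.
; Align spawns an INT anchor at the player camera and creates its anchor from the given transform.
; It spawns an attached EXT anchor at that transform, pairs both, then runs the component's alignment.
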(event `EnhancedInput|/LASAA/InputActions/IA_ResetAnchors`
  (params (ActionValue :type Boolean) (ElapsedSeconds :type "Float (double-precision)") (TriggeredSeconds :type "Float (double-precision)") (InputAction :type "InputAction Object Reference" :default "/LASAA/InputActions/IA_ResetAnchors.IA_ResetAnchors"))
  ;[1 1 1] Reset all anchors
  (:`Triggered`
    (`Anchor.resetAnchors`)))

(event `EnhancedInput|/LASAA/InputActions/IA_PlaceAnchor`
  (params (ActionValue :type Boolean) (ElapsedSeconds :type "Float (double-precision)") (TriggeredSeconds :type "Float (double-precision)") (InputAction :type "InputAction Object Reference" :default "/LASAA/InputActions/IA_PlaceAnchor.IA_PlaceAnchor"))
  ;[1 1 1] Place a new anchor
  (:`Triggered`
    (`self.RequestPlaceAnchor`)))

(event `self.ReceiveBeginPlay`
  ;[1 1 1] Init alignment component
  (bind _returnvalue (`AddComponent|NODE_AddAlignmentComponent-0`))
  (`AlignmentComponent.configureAlignmentComponent` _returnvalue (`self.INTAnchorClass`) (`self.EXTAnchorClass`) 1 false)
  (set `self.AlignComp` _returnvalue)
  (set `self.PlayerCamera` (`self.GetComponentByClass` (`GameplayStatics.GetPlayerPawn` 0) "/Script/Engine.CameraComponent")))

(fn `Align`
  (params (AnchorTransform :type "Transform Structure"))
  (returns (Aligned :type Boolean))
  (bind _returnvalue (`|SpawnActorFromClass` (`self.INTAnchorClass`) (`SceneComponent.K2_GetComponentToWorld` (`self.PlayerCamera`)) "AlwaysSpawn" "MultiplyWithRoot" null null))
  (`Anchor.createAnchor` _returnvalue AnchorTransform)
  (bind _returnvalue_2 (`|SpawnActorFromClass` (`self.EXTAnchorClass`) AnchorTransform "AlwaysSpawn" "MultiplyWithRoot" null null))
  (`self.K2_AttachToActor` _returnvalue_2 self "None" "KeepRelative" "KeepRelative" "KeepRelative" false)
  (`Anchor.setExtPairAndCalibrationOffset` _returnvalue _returnvalue_2)
  (bind _returnvalue_3 (`AlignmentComponent.align` (`self.AlignComp`)))
  (return _returnvalue_3))

(fn `RequestPlaceAnchor`
  (set `self.PlaceAnchor` true))

(fn `UserConstructionScript`)