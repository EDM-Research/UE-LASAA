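; AnchorsConfig is a configuration Blueprint that sets up the anchor system at BeginPlay for either a preparation or an operational stage.
; With PreparationStage set, it spawns an AnchorPlacer at the origin, passing the interior/exterior anchor classes and AnchorBuffer.
; Otherwise, it adds and configures a ticking alignment component on AnchorParent, then calls AddChangeMode on Player.
; A MinNumberMatches assignment to the spawned placer is left unconnected and never runs.
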(event `self.ReceiveBeginPlay`
  (if (`self.Preparation stage`)
    ;[1 1 1] Setup for preparation stage
    (bind _returnvalue (`|SpawnActorFromClass` "/LASAA/Blueprints/AnchorPlacer.AnchorPlacer_C" (`KismetMathLibrary.MakeTransform` (0.0 0.0 0.0)) "Undefined" "MultiplyWithRoot" null (`self.INTAnchorClass`) (`self.EXTAnchorClass`) (`self.AnchorBuffer`) null))
    (else
      ;[1 1 1] Setup for operational stage
      (bind _returnvalue_2 (`AddComponent|NODE_AddAlignmentComponent-1` :`self` (`self.AnchorParent`) :`anchorBuffer` (`self.AnchorBuffer`)))
      (`AlignmentComponent.configureAlignmentComponent` _returnvalue_2 (`self.INTAnchorClass`) (`self.EXTAnchorClass`) (`self.AlignmentMode`) true)
      (`AddComponent|NODE_AddChangeMode-1` :`self` (`self.Player`)))))

(fn `UserConstructionScript`)