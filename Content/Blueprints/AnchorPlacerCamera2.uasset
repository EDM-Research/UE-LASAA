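; AnchorPlacerCamera2 is an anchor placer that aligns to an anchor pose received over OSC from a processing device.
; On BeginPlay it sends camera calibration to the device's OSC client and starts an OSC server on port 8001.
; Placement requests ask the device for a pose.
; Incoming messages are used only while a placement is pending, clearing that flag, and call Align only if tracking state is zero and the transform parses.
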(event `self.ReceiveBeginPlay`
  ;[1 1 1] Setup
  (`parent.ReceiveBeginPlay`)
  (`|ExecutionSequence`
    (:`then_0`
      (bind _returnvalue (`Helper.CreateProcessingDeviceOSCClient` self))
      (bind _output_get (set `self.OSCClient` _returnvalue))
      (`Helper.GetAndSendCameraCalibrationToClient` _output_get))
    (:`then_1`
      (bind _returnvalue_2 (`OSCManager.CreateOSCServer` "" 8001 false true "" self))
      (bind _output_get_2 (set `self.OSCServer` _returnvalue_2))
      (add `OSCServer.OnOscMessageReceived` _output_get_2 (delegate `OnOscMessageReceivedEvent`)))))

(event `OnOscMessageReceivedEvent`
  (params (Message :type "OSCMessage Structure (by ref)") (IPAddress :type String) (Port :type Integer))
  ;[1 1 1] On OSC received -> get anchors
  ;;[1 1 1] Only continue when an anchor needs to be placed, and if tracking state is 0
  (if (`self.PlaceAnchor`)
    (set `self.PlaceAnchor` false)
    (bind _value (`OSCManager.GetInt32` Message))
    (if (== _value 0)
      (bind (_anchortransform _returnvalue) (`Helper.GetAnchorTransformFromOSCMessage` Message))
      (if _returnvalue
        (`self.Align` _anchortransform)))))

(fn `RequestPlaceAnchor`
  (`parent.RequestPlaceAnchor`)
  (`Helper.SendRequestForAnchorPoseToClient` (`self.OSCClient`)))

(fn `UserConstructionScript`)