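; Input-driven debug Blueprint that switches the anchor alignment mode and cycles the opacity of meshes.
; The align action calls ChangeMode on the AlignmentComponent of the AnchorsConfig actor's AnchorParent and prints the result.
; The opacity action steps a material parameter collection scalar through transparent, half and full, then sets the slot 0 material on static meshes of MESH-tagged actors, printing opaque or translucent.
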(event `EnhancedInput|/LASAA/InputActions/IA_AlignMode`
  (params (ActionValue :type Boolean) (ElapsedSeconds :type "Float (double-precision)") (TriggeredSeconds :type "Float (double-precision)") (InputAction :type "InputAction Object Reference" :default "/LASAA/InputActions/IA_AlignMode.IA_AlignMode"))
  ;[1 1 1] Change the alignment mode (weighted - static)
  (:`Triggered`
    (bind _returnvalue (`GameplayStatics.GetActorOfClass` "/LASAA/Blueprints/AnchorsConfig.AnchorsConfig_C"))
    (bind _returnvalue_2 (`AlignmentComponent.changeMode` (`Actor.GetComponentByClass` (`/LASAA/Blueprints/AnchorsConfig.AnchorParent` _returnvalue) "/Script/LASAA.AlignmentComponent")))
    (`KismetSystemLibrary.PrintString` (`KismetStringLibrary.Concat_StrStr` " \n \n \n \n \n \n                                                                                                                                              " _returnvalue_2))))

(event `EnhancedInput|/LASAA/InputActions/IA_ChangeOpacity`
  (params (ActionValue :type Boolean) (ElapsedSeconds :type "Float (double-precision)") (TriggeredSeconds :type "Float (double-precision)") (InputAction :type "InputAction Object Reference" :default "/LASAA/InputActions/IA_ChangeOpacity.IA_ChangeOpacity"))
  (bind _returnvalue (mod (+ (`self.index`) 1) 3))
  ;[1 1 1] Change opacity
  (:`Triggered`
    (`KismetMaterialLibrary.SetScalarParameterValue` "/LASAA/Other/Opacity.Opacity" "OpacityMesh" (select `int` _returnvalue :`0` 0.0 :`1` 0.5 :`2` 1.0 :!type "Float (single-precision)"))
    (bind _output_get (set `self.index` _returnvalue))
    (bind _outactors (`GameplayStatics.GetAllActorsWithTag` "MESH"))
    (for _array_element _outactors
      (for _array_element_2 (`Actor.K2_GetComponentsByClass` _array_element "/Script/Engine.StaticMeshComponent")
        (if (== _output_get 2)
          (`PrimitiveComponent.SetMaterial` _array_element_2 0 null)
          (`KismetSystemLibrary.PrintText` "opaque")
          (else
            (`PrimitiveComponent.SetMaterial` _array_element_2 0 null)
            (`KismetSystemLibrary.PrintText` "translucent")))))))